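; Door actor that opens for Tantrumn AI enemy characters when they enter its box trigger.
; Overlap begin sets the open flag if the door is closed and calls GoToAndOpenDoor on the enemy; overlap end clears it.
; Tick polls the open state and toggles the mesh's visibility and collision instead of animating it.
; A timeline-driven rotation swing is present but unconnected.
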(event OnComponentBeginOverlap(BoxCollision)
  (params (OverlappedComponent :type Primitive%20Component%20Object%20Reference) (OtherActor :type Actor%20Object%20Reference) (OtherComp :type Primitive%20Component%20Object%20Reference) (OtherBodyIndex :type Integer) (bFromSweep :type Boolean) (SweepResult :type Hit%20Result%20Structure%20%28by%20ref%29))
  (bind _asbp_tantrumn_enemy_character_ai (Utilities|Casting|CastToBP_TantrumnEnemyCharacterAI OtherActor))
  (bind _returnvalue (Class|Door|GetDoorIsOpen))
  (if (not _returnvalue)
    (Variables|Default|SetbIsOpen true)
    (Default|GotoandOpenDoor _asbp_tantrumn_enemy_character_ai)))

(event OnComponentEndOverlap(BoxCollision)
  (params (OverlappedComponent :type Primitive%20Component%20Object%20Reference) (OtherActor :type Actor%20Object%20Reference) (OtherComp :type Primitive%20Component%20Object%20Reference) (OtherBodyIndex :type Integer))
  (Utilities|Casting|CastToBP_TantrumnEnemyCharacterAI OtherActor)
  (Variables|Default|SetbIsOpen false))

(event EventTick
  (params (DeltaSeconds :type Float%20%28single-precision%29))
  (bind _returnvalue (Class|Door|GetDoorIsOpen))
  (if _returnvalue
    (Rendering|SetVisibility (Variables|Default|GetDoorMesh) false false)
    (Collision|SetCollisionEnabled (Variables|Default|GetDoorMesh) "NoCollision")
    (else
      (Rendering|SetVisibility (Variables|Default|GetDoorMesh) true false)
      (Collision|SetCollisionEnabled (Variables|Default|GetDoorMesh) "QueryAndPhysics"))))

(fn ConstructionScript)