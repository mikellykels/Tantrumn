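; Base character Blueprint for Tantrumn, whose event graph is now inert, with a note that it was converted to C++.
; Disconnected leftover nodes would create a name widget and show the name of an attached throwable via an interface, clearing it otherwise.
; A Hold macro separates Tap from Held using two gates and a retriggerable delay: early release fires Tap, while reaching the duration fires Held.
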(event Custom|GetObjectName
  ;[0 0.8102 1] Converted to C++
  ;;[1 1 1] Get the name of attached actor
)

(event EventBeginPlay
  ;[0 0.8102 1] Converted to C++
  ;;[1 1 1] Display Name Widget for equipped ball
)

(event EventTick
  (params (DeltaSeconds :type Float%20%28single-precision%29))
  ;[0 0.8102 1] Converted to C++
  ;;[1 1 1] Check if throwable actor is attached to character
)

(fn ConstructionScript)