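; Enemy AI character for Tantrumn that seeks out a door and walks through it on BeginPlay.
; It scans BP_Door actors with a growing distance threshold, then chains AIMoveTo from the door's nearer reference point to the far one, pausing between.
; On reaching a jump link, it launches itself using ballistic velocity math expressions.
; A Blackboard-based version of the door movement is left disconnected.
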(event Custom|FindNearestDoor
  (Variables|Default|SetSearchingForDoor true)
  (bind _outactors (Actor|GetAllActorsOfClass "/Game/Tantrumn/Blueprints/Actors/BP_Door.BP_Door_C"))
  (bind _array_element (Utilities|Array|ForEachLoopwithBreak _outactors :!label _label)
    (:LoopBody
      (if (<= (Transformation|GetDistanceTo _array_element) (Variables|Default|GetDistance))
        (Variables|Default|SetSearchingForDoor false)
        (Variables|Default|SetDistance 1e+02)
        (Variables|Default|SetDoorRef _array_element)
        (goto _label Break)
        (else
          (Variables|Default|SetDistance (+ (Variables|Default|GetDistance) 5e+01)))))
    (:Completed
      (if (Variables|Default|GetSearchingForDoor)
        (goto _label)
        (else
          (CallFunction|GotoandOpenDoor))))))

(event Custom|GoToAndOpenDoor
  (bind _returnvalue (Transformation|GetActorLocation))
  (bind _self self)
  (bind _self_2 self)
  (bind _doorref (Variables|Default|GetDoorRef))
  (bind _openref1 (Variables|/Game/Tantrumn/Blueprints/Actors/BP_Door.BP_Door_C|GetOpenREF1 _doorref))
  (bind _openref2 (Variables|/Game/Tantrumn/Blueprints/Actors/BP_Door.BP_Door_C|GetOpenREF2 _doorref))
  (bind _returnvalue_2 (Transformation|GetWorldLocation _openref1))
  (bind _returnvalue_3 (Transformation|GetWorldLocation _openref2))
  (if (< (Math|Vector|VectorLength (- _returnvalue _returnvalue_2)) (Math|Vector|VectorLength (- _returnvalue _returnvalue_3)))
    (AI|AIMoveTo _self _returnvalue_2 0 5.0 false
      (:OnSuccess
        (Utilities|FlowControl|Delay 1.0)
        (Development|PrintString "REFA")
        (AI|AIMoveTo _self_2 _returnvalue_3 0 5.0 false
          (:OnSuccess
            (bind _output_get (Variables|Default|SetWentThroughDoor true))
            (Development|PrintString (Utilities|String|ToString(Boolean) _output_get))))))
    (else
      (AI|AIMoveTo _self _returnvalue_3 0 5.0 false
        (:OnSuccess
          (Utilities|FlowControl|Delay 1.0)
          (Development|PrintString "REFB")
          (AI|AIMoveTo _self_2 _returnvalue_2 0 5.0 false
            (:OnSuccess
              (bind _output_get_2 (Variables|Default|SetWentThroughDoor true))
              (Development|PrintString (Utilities|String|ToString(Boolean) _output_get_2)))))))))

(event EventJumpLinkReached
  (params (JumpLinkProxyDestination :type Vector :default "0, 0, 0"))
  (bind _returnvalue (Transformation|GetActorLocation))
  (bind (_x _y _z) (Math|Vector|BreakVector JumpLinkProxyDestination))
  (bind (_x_2 _y_2 _z_2) (Math|Vector|BreakVector _returnvalue))
  (Character|LaunchCharacter (Math|Vector|MakeVector (|((DestinationX-StartX)/{091C5CEA-43CE-2444-FABE-B7A07EAB006A}) _x _x_2) (|((DestinationY-StartY)/{091C5CEA-43CE-2444-FABE-B7A07EAB006A}) _y _y_2) (|((DestinationHeight-(StartHeight-(((Power({091C5CEA-43CE-2444-FABE-B7A07EAB006A},2))*0.500000)*{E32FEC85-4BF5-9858-0101-598235585722})))/{091C5CEA-43CE-2444-FABE-B7A07EAB006A}) _z _z_2)) true true))

(event EventBeginPlay
  (CallFunction|FindNearestDoor))

(fn ConstructionScript)