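; Behavior tree task for Tantrumn's enemy AI that reports whether the controlled enemy has gone through a door.
; On execute it casts the pawn to BP_TantrumnEnemyCharacterAI and finishes with success or failure from its WentThroughDoor flag, printing debug messages along the way.
; A failed cast only prints, leaving the task unfinished.
; The calls to find, approach and open a door are disconnected, so the task itself moves nothing.
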(event EventReceiveExecuteAI
  (params (OwnerController :type AI%20Controller%20Object%20Reference) (ControlledPawn :type Pawn%20Object%20Reference))
  (Development|PrintString "EXECUTE")
  (bind _asbp_tantrumn_enemy_character_ai (Utilities|Casting|CastToBP_TantrumnEnemyCharacterAI ControlledPawn)
    (:then
      (Development|PrintString (Utilities|String|ToString(Boolean) (Variables|/Game/Tantrumn/Blueprints/Characters/BP_TantrumnEnemyCharacterAI.BP_TantrumnEnemyCharacterAI_C|GetWentThroughDoor _asbp_tantrumn_enemy_character_ai)) true true "(R=1.000000,G=0.000000,B=0.464954,A=1.000000)")
      (if (Variables|/Game/Tantrumn/Blueprints/Characters/BP_TantrumnEnemyCharacterAI.BP_TantrumnEnemyCharacterAI_C|GetWentThroughDoor _asbp_tantrumn_enemy_character_ai)
        (AI|BehaviorTree|FinishExecute true)
        (Development|PrintString "FINISH EXECUTE")
        (else
          (AI|BehaviorTree|FinishExecute false)
          (Development|PrintString "DID NOT FINISH"))))
    (:CastFailed
      (Development|PrintString "CAST FAILED"))))